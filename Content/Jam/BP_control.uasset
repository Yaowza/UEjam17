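; RTS-style player controller that shows the mouse cursor, locks it to the viewport and handles unit selection and move orders.
; Left mouse press, hold and release send marquee messages to the HUD, with Tick driving the held state.
; Right click traces under the cursor, orders the HUD's selected units to that point and spawns a Niagara click effect.
; A HandleBuilding function, not called here, selects and stores the building under the cursor.
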(event EventBeginPlay
  (Input|SetInputModeGameandUI self 0 "LockAlways" false)
  (Variables|Default|SetbShowMouseCursor true))

(event EventTick
  (params (DeltaSeconds :type Float%20%28single-precision%29))
  (if (Variables|Default|Getlftmouspressed?)
    (Class|RTXinterface|Marqueheld(Message) (HUD|GetHUD))))

(event Input|MouseEvents|LeftMouseButton
  (params (Key :type Key%20Structure :default "None"))
  (bind _returnvalue (HUD|GetHUD))
  (:Pressed
    (Variables|Default|Setlftmouspressed? true)
    (Class|RTXinterface|Marquepressed(Message) _returnvalue))
  (:Released
    (Variables|Default|Setlftmouspressed? false)
    (Class|RTXinterface|Marquereleased(Message) _returnvalue)))

(event Input|MouseEvents|RightMouseButton
  (params (Key :type Key%20Structure :default "None"))
  (:Pressed
    (Variables|Default|Setpall true)
    (Variables|Default|Set%20rich%20click%20location (.Location (Collision|BreakHitResult (.HitResult (Game|Player|GetHitResultUnderCursorbyChannel "TraceTypeQuery1" true)))))
    (bind _limits (Class|RTXinterface|Grabselectedunits(Message) (HUD|GetHUD)))
    (for _array_element _limits
      (Class|RTXinterface|Unitmovecommand(Message) _array_element (Variables|Default|Get%20rich%20click%20location)))
    (Niagara|SpawnSystematLocation "/Game/Cursor/FX_Cursor.FX_Cursor" (Variables|Default|Get%20rich%20click%20location))))

(fn ConstructionScript)

(fn Grabselectedunits
  (return 0))