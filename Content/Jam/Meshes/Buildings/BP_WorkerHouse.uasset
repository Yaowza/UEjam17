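; BP_WorkerHouse is a worker house building that spawns a Fourmiz_classe1 actor at its own transform on BeginPlay.
; Placement functions paint every StaticMesh material slot with a green or red placement material and clear IsActive, while SetMashMaterials restores the stored MeshMaterial array.
; SetGreenPlacement and SetRedPlacement apply the opposite color to their names, and Ahh is another green-painting loop.
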(event EventBeginPlay
  (Game|SpawnActorfromClass "/Game/Jam/fourmiz1/Fourmiz_classe1.Fourmiz_classe1_C" (Transformation|GetActorTransform) "AlwaysSpawn" 0 0))

(fn ConstructionScript)

(fn Ahh
  (for _index (range 0 (Utilities|Array|LastIndex (Utilities|Array|MakeArray 0)))
    (Rendering|Material|SetMaterial (Variables|Default|GetStaticMesh) _index "/Game/Jam/Materials/Feedback/GreenPlacement.GreenPlacement")))

(fn SetGreenPlacement
  (for _index (range 0 (Utilities|Array|LastIndex (Variables|Default|GetMeshMaterial)))
    (Rendering|Material|SetMaterial (Variables|Default|GetStaticMesh) _index "/Game/Jam/Materials/Feedback/RedPlacement.RedPlacement"))
  (Variables|Default|SetIsActive false))

(fn SetMashMaterials
  (for (_array_element _array_index) (Variables|Default|GetMeshMaterial)
    (Rendering|Material|SetMaterial (Variables|Default|GetStaticMesh) _array_index _array_element)))

(fn SetRedPlacement
  (for _index (range 0 (Utilities|Array|LastIndex (Variables|Default|GetMeshMaterial)))
    (Rendering|Material|SetMaterial (Variables|Default|GetStaticMesh) _index "/Game/Jam/Materials/Feedback/GreenPlacement.GreenPlacement"))
  (Variables|Default|SetIsActive false))